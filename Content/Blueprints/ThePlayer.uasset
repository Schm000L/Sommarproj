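; Player character for a 2D Paper2D side-scroller with double jump, crouch, ledge hanging and mouse-aimed weapons.
; Tick checks HP, rotates weapon and body toward the cursor, and runs height and wall sphere traces for ledge grabs.
; Weapon sprite, projectile, sound and fire delay come from the WeaponData table, while an enum state selects flipbooks.
; Crouch presses also subtract HP, and debug traces are drawn.
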(event OnComponentBeginOverlap(CircleTracer)
  (params (OverlappedComponent :type Primitive%20Component%20Object%20Reference) (OtherActor :type Actor%20Object%20Reference) (OtherComp :type Primitive%20Component%20Object%20Reference) (OtherBodyIndex :type Integer) (bFromSweep :type Boolean) (SweepResult :type Hit%20Result%20Structure%20%28by%20ref%29))
  ;[1 1 1] Ledges
  ;;[1 1 1] Can Trace Event
  (Variables|Ledge|SetCanTrace true))

(event OnComponentEndOverlap(CircleTracer)
  (params (OverlappedComponent :type Primitive%20Component%20Object%20Reference) (OtherActor :type Actor%20Object%20Reference) (OtherComp :type Primitive%20Component%20Object%20Reference) (OtherBodyIndex :type Integer))
  ;[1 1 1] Ledges
  ;;[1 1 1] Can Trace Event
  (Variables|Ledge|SetCanTrace false))

(event Custom|UpdateAnimation
  (bind _charactermovement (Variables|Character|GetCharacterMovement))
  ;[1 1 1] Set variables for flipbook
  (Variables|Movement|SetIsMoving (> (Math|Vector|VectorLength (Transformation|GetVelocity)) 0.0)) ; Custom Variable
  (Variables|Movement|SetIsFalling (AI|Components|NavMovement|IsFalling _charactermovement))
  (Variables|Movement|SetIsCrouching (AI|Components|NavMovement|IsCrouching _charactermovement))
  ;[1 1 1] Change player flipbook
  (bind _outputflipbook (CallFunction|AnimationStateMachine (Variables|Default|GetbIsCrouched) (Variables|Movement|GetIsFalling) (Variables|Movement|GetIsMoving) (Variables|Ledge|GetIsHanging)))
  (Sprite|SetFlipbook (Variables|Default|GetSprite) _outputflipbook))

(event Custom|ResetBlockShooting
  ;[1 1 1] Fire
  (Utilities|FlowControl|DoOnce false) ; enters at Reset
)

(event Custom|CheckHP
  ;[1 1 1] Health
  (if (<= (Variables|Health|GetCurrentHP) 0.0)
    (Actor|DestroyActor)))

(event Custom|UpdatePlayerRotation
  (bind _returnvalue (Math|Rotator|MakeRotator 0.0 0.0 1.8e+02))
  ;[1 1 1] Rotate player
  (Math|Float|CompareFloat (Variables|Mouse|GetMouseXRelativeToPlayer) 0.0
    (:>
      (Pawn|SetControlRotation (Pawn|GetController) (Math|Rotator|MakeRotator 0.0 0.0 0.0)) ; Flippa inte sprite
    )
    (:<
      (Pawn|SetControlRotation (Pawn|GetController) _returnvalue) ; Flippa sprite
      (Variables|Mouse|SetMouseRotation (Math|Rotator|CombineRotators (Variables|Mouse|GetMouseRotation) _returnvalue)))))

(event Custom|HandleLedgeTick
  (bind (_start _end) (Utilities|WallTracer))
  (bind (_start_2 _end_2) (Utilities|LedgeTracer 3e+02))
  ;[1 1 1] Ledges
  (if (Variables|Ledge|GetCanTrace)
    (Utilities|FlowControl|Sequence
      (:then_0
        ;;[1 1 1] Ledge Height Tracer
        (bind (_outhit _returnvalue) (Collision|SphereTraceByChannel _start_2 _end_2 0.0 "TraceTypeQuery3" false (Utilities|Array|MakeArray 0) "ForOneFrame"))
        (if _returnvalue
          (Variables|Ledge|SetLedgeHeight (.ImpactPoint (Collision|BreakHitResult _outhit)))))
      (:then_1
        ;;[1 1 1] Wall Tracer
        (bind (_outhit_2 _returnvalue_2) (Collision|SphereTraceByChannel _start _end 2e+01 "TraceTypeQuery3" false (Utilities|Array|MakeArray 0) "ForOneFrame"))
        (if _returnvalue_2
          (Variables|Ledge|SetWallTraceImpact (.ImpactPoint (Collision|BreakHitResult _outhit_2)))
          (Variables|Ledge|SetWallNormal (.ImpactNormal (Collision|BreakHitResult _outhit_2)))
          ;;[1 1 1] Grab ledge
          (if (and (Math|Float|InRange(Float) (- (.Z (Math|Vector|BreakVector (Variables|Ledge|GetLedgeHeight))) (.Z (Math|Vector|BreakVector (Transformation|GetActorLocation)))) 0.0 (Variables|Ledge|GetMaxGrabDistance%20%28z-axis%29)) (Variables|Ledge|GetCanGrab))
            (Pawn|Components|CharacterMovement|SetMovementMode (Variables|Character|GetCharacterMovement) "MOVE_Flying" 0)
            (Variables|Ledge|SetIsHanging true)
            (Variables|Ledge|SetCanGrab false)
            (Components|MoveComponentTo (Variables|Collision|GetCapsuleComponent) (Utilities|WallGotoLocation) (Transformation|GetActorRotation) false false 0.2 false)
            (Components|Movement|StopMovementImmediately (Variables|Character|GetCharacterMovement))
            (CallFunction|UpdateAnimation)))))))

(event Custom|UpdateWeaponRotation
  (bind _returnvalue (Viewport|GetViewportSize))
  (bind _returnvalue_2 (Game|GetPlayerController 0))
  (bind (_x _y) (Math|Vector2D|BreakVector2D _returnvalue))
  (bind (_locationx _locationy) (Game|Player|GetMousePosition _returnvalue_2))
  ;[1 1 1] Rotate weapon
  (bind _output_get (Variables|Mouse|SetMouseXRelativeToPlayer (- _locationx (/ _x 2.0))))
  (bind _output_get_2 (Variables|Mouse|SetMouseYRelativeToPlayer (- (/ _y 2.0) _locationy)))
  (Transformation|SetRelativeRotation (Variables|Weapon|GetCurrentWeaponSprite) (Math|Rotator|MakeRotator 0.0 (Class|KismetMathLibrary|DegAtan2 _output_get_2 (Math|Float|Absolute(Float) _output_get)) 0.0) false false)
  (Variables|Mouse|SetMouseRotation (Math|Rotator|CombineRotators (Math|Rotator|MakeRotator 0.0 (Class|KismetMathLibrary|DegAtan2 _output_get_2 (Math|Float|Absolute(Float) _output_get)) 0.0) (* (Pawn|GetControlRotation :!class /Script/Engine.Pawn) 2.0))))

(event Custom|BlockShooting
  ;[1 1 1] Fire
  (bind _weapondelay (Weapon|GetWeaponDelay (Variables|Weapon|GetCurrentWeapon)))
  (Utilities|FlowControl|Delay _weapondelay)
  (CallFunction|ResetBlockShooting))

(event Custom|Let%20go%20of%20ledge
  ;[1 1 1] Ledges
  ;;[1 1 1] Let go of ledge
  (if (Variables|Ledge|GetIsHanging)
    (Pawn|Components|CharacterMovement|SetMovementMode (Variables|Character|GetCharacterMovement) "MOVE_Walking" 0)
    (Variables|Ledge|SetIsHanging false)
    (Utilities|FlowControl|Delay 0.5)
    (Variables|Ledge|SetCanGrab true)))

(event Collision|EventActorBeginOverlap
  (params (OtherActor :type Actor%20Object%20Reference))
  ;[1 1 1] Will be used for pickups later
)

(event EventBeginPlay
  (bind _returnvalue (Game|GetPlayerController 0))
  ;[1 1 1] Setup stuff before start
  ;[1 1 1] Add weapon to player
  (bind _returnvalue_2 (AddComponent|AddPaperSpriteComponent false))
  (Variables|Weapon|SetCurrentWeaponSprite _returnvalue_2)
  ;[1 1 1] Display cursor
  (Variables|/Script/Engine.PlayerController|SetbShowMouseCursor _returnvalue true)
  (Variables|/Script/Engine.PlayerController|SetCurrentMouseCursor _returnvalue "Crosshairs")
  (bind _returnvalue_3 (UserInterface|CreateWidget "/Game/Blueprints/WidgetHUD.WidgetHUD_C"))
  (UserInterface|Viewport|AddtoViewport _returnvalue_3 0))

(event EventOnLanded
  (params (Hit :type Hit%20Result%20Structure%20%28by%20ref%29))
  ;[1 1 1] Jumping
  (Variables|Movement|SetJumps 2)
  (Utilities|FlowControl|DoN (Variables|Movement|GetJumps)) ; enters at Reset
)

(event EventTick
  (params (DeltaSeconds :type Float%20%28single-precision%29))
  ;[1 1 1] Game tick events
  ;[1 1 1] Check HP
  (CallFunction|CheckHP)
  ;[1 1 1] Rotates weapon
  (CallFunction|UpdateWeaponRotation)
  ;[1 1 1] Rotate player
  (CallFunction|UpdatePlayerRotation)
  ;[1 1 1] Trace ledges
  (CallFunction|HandleLedgeTick))

(event EventOnWalkingOffLedge
  (params (PreviousFloorImpactNormal :type Vector%20%28by%20ref%29 :default "0, 0, 0") (PreviousFloorContactNormal :type Vector%20%28by%20ref%29 :default "0, 0, 0") (PreviousLocation :type Vector%20%28by%20ref%29 :default "0, 0, 0") (TimeDelta :type Float%20%28single-precision%29))
  ;[1 1 1] Jumping
  (Variables|Movement|SetJumps 1))

(event Input|ActionEvents|InputActionJump
  (params (Key :type Key%20Structure :default "AnyKey"))
  ;[1 1 1] Jumping
  (:Pressed
    (if (not (Variables|Movement|GetIsCrouching))
      (if (Variables|Ledge|GetIsHanging)
        (CallFunction|LetGoOfLedge)
        (Utilities|FlowControl|Sequence
          (:then_0
            (goto _label Reset))
          (:then_1
            _)))
      (bind _counter (Utilities|FlowControl|DoN (Variables|Movement|GetJumps) :!label _label)
        (:Exit
          (switch int _counter
            (:1
              _)
            (:2
              _))
          (if (Variables|Movement|GetIsFalling)
            (Character|LaunchCharacter "0,0.000000,1000.000000" false true)
            (else
              (Character|Jump))))))))

(event Input|ActionEvents|InputActionCrouch
  (params (Key :type Key%20Structure :default "AnyKey"))
  ;[1 1 1] Crouching
  (:Pressed
    (if (Variables|Ledge|GetIsHanging)
      (CallFunction|LetGoOfLedge)
      (else
        (Character|Crouch)
        (Variables|Health|SetCurrentHP (- (Variables|Health|GetCurrentHP) 25.0)))))
  (:Released
    (Character|UnCrouch)))

(event Input|ActionEvents|InputActionPistol
  (params (Key :type Key%20Structure :default "AnyKey"))
  ;[1 1 1] Change weapon
  (:Pressed
    (Variables|Weapon|SetWeaponToCheck "NewEnumerator0")
    (Weapon|ChangeWeapon (Variables|Weapon|GetWeaponToCheck))))

(event Input|ActionEvents|InputActionShotgun
  (params (Key :type Key%20Structure :default "AnyKey"))
  ;[1 1 1] Change weapon
  (:Pressed
    (Variables|Weapon|SetWeaponToCheck "NewEnumerator1")
    (Weapon|ChangeWeapon (Variables|Weapon|GetWeaponToCheck))))

(event Input|ActionEvents|InputActionSMG
  (params (Key :type Key%20Structure :default "AnyKey"))
  ;[1 1 1] Change weapon
  (:Pressed
    (Variables|Weapon|SetWeaponToCheck "NewEnumerator2")
    (Weapon|ChangeWeapon (Variables|Weapon|GetWeaponToCheck))))

(event Input|ActionEvents|InputActionRifle
  (params (Key :type Key%20Structure :default "AnyKey"))
  ;[1 1 1] Change weapon
  (:Pressed
    (Variables|Weapon|SetWeaponToCheck "NewEnumerator3")
    (Weapon|ChangeWeapon (Variables|Weapon|GetWeaponToCheck))))

(event Input|ActionEvents|InputActionGrenadeLauncher
  (params (Key :type Key%20Structure :default "AnyKey"))
  ;[1 1 1] Change weapon
  (:Pressed
    (Variables|Weapon|SetWeaponToCheck "NewEnumerator7")
    (Weapon|ChangeWeapon (Variables|Weapon|GetWeaponToCheck))))

(event Input|ActionEvents|InputActionCrossbow
  (params (Key :type Key%20Structure :default "AnyKey"))
  ;[1 1 1] Change weapon
  (:Pressed
    (Variables|Weapon|SetWeaponToCheck "NewEnumerator8")
    (Weapon|ChangeWeapon (Variables|Weapon|GetWeaponToCheck))))

(event Input|ActionEvents|InputActionSword
  (params (Key :type Key%20Structure :default "AnyKey"))
  ;[1 1 1] Change weapon
  (:Pressed
    (Variables|Weapon|SetWeaponToCheck "NewEnumerator9")
    (Weapon|ChangeWeapon (Variables|Weapon|GetWeaponToCheck))))

(event Input|AxisEvents|InputAxisMoveRight
  (params (AxisValue :type Float%20%28single-precision%29))
  ;[1 1 1] Running
  (if (not (Variables|Ledge|GetIsHanging))
    (Pawn|Input|AddMovementInput "1.000000, 0, 0" AxisValue false) ; Flytta karaktär
    ;[1 1 1] Flip the flipbook (not used)
    (CallFunction|UpdateAnimation)))

(event Input|AxisEvents|InputAxisFire
  (params (AxisValue :type Float%20%28single-precision%29))
  ;[1 1 1] Fire
  (if (Math|Conversions|ToBoolean(Integer) (Math|Float|Truncate AxisValue))
    (Utilities|FlowControl|DoOnce false
      (:Completed
        (Weapon|Fire (Variables|Weapon|GetCurrentWeapon))
        (CallFunction|BlockShooting)))))

(fn ConstructionScript)

(fn AnimationStateMachine
  (params (IsCrouching :type Boolean) (IsFalling :type Boolean) (IsMoving :type Boolean) (IsLedgeGrabbing :type Boolean))
  ;[1 1 1] Branch from inputs
  (if IsCrouching
    (if IsMoving
      ;[1 1 1] Set AnimationState
      (LocalVariables|SetAnimationState "NewEnumerator3")
      (else
        (LocalVariables|SetAnimationState "NewEnumerator4")))
    (elif IsFalling
      (LocalVariables|SetAnimationState "NewEnumerator2")
      (elif IsMoving
        (LocalVariables|SetAnimationState "NewEnumerator1")
        (elif IsLedgeGrabbing
          (LocalVariables|SetAnimationState "NewEnumerator5")
          (else
            (LocalVariables|SetAnimationState "NewEnumerator0"))))))
  (return (Utilities|Select :Index (LocalVariables|GetAnimationState) :NewEnumerator0 (Variables|Animations|GetIdleFlipbook) :NewEnumerator1 (Variables|Animations|GetRunFlipbook) :NewEnumerator2 (Variables|Animations|GetJumpFlipbook) :NewEnumerator3 (Variables|Animations|GetCrouchFlipbook) :NewEnumerator4 (Variables|Animations|GetIdleCrouchFlipbook) :NewEnumerator5 (Variables|Animations|GetLedgeGrabbingFlipbook))))

(fn Fire
  (params (CurrentWeapon :type Weapons%20Enum))
  ;[1 1 1] Get weapon info
  (bind _outrow (Weapon|GetDatafromWeapon CurrentWeapon))
  ;[1 1 1] Spawn bullet
  (Game|SpawnActorfromClass (.BulletClass (Utilities|Struct|BreakWeaponStruct _outrow)) (Math|Transform|MakeTransform (Transformation|GetActorLocation) (Variables|Mouse|GetMouseRotation)) "Undefined" 0 0)
  ;[1 1 1] Play a gun sound
  (Audio|SpawnSoundatLocation (.FireSound (Utilities|Struct|BreakWeaponStruct _outrow)) (Transformation|GetActorLocation)))

(fn GetWeaponDelay
  (params (CurrentWeapon :type Weapons%20Enum))
  (bind _outrow (Weapon|GetDatafromWeapon CurrentWeapon))
  (return (.Delay (Utilities|Struct|BreakWeaponStruct _outrow))))

(fn GetNextWeapon
  (params (CurrentWeapon :type Weapons%20Enum))
  ;[1 1 1] Sorry
  (switch Utilities|FlowControl|Switch|SwitchonWeapons CurrentWeapon
    (:NewEnumerator0
      (LocalVariables|SetNextWeapon "NewEnumerator1"))
    (:NewEnumerator1
      (LocalVariables|SetNextWeapon "NewEnumerator2"))
    (:NewEnumerator2
      (LocalVariables|SetNextWeapon "NewEnumerator3"))
    (:NewEnumerator3
      (LocalVariables|SetNextWeapon "NewEnumerator7"))
    (:NewEnumerator7
      (LocalVariables|SetNextWeapon "NewEnumerator8"))
    (:NewEnumerator8
      (LocalVariables|SetNextWeapon "NewEnumerator9"))
    (:NewEnumerator9
      (LocalVariables|SetNextWeapon "NewEnumerator0")))
  (return (LocalVariables|GetNextWeapon)))

(fn ChangeWeapon
  (params (NewWeapon :type Weapons%20Enum))
  ;[1 1 1] Check if player has weapon unlocked (not used anymore)
  (bind _outrow (Weapon|GetDatafromWeapon NewWeapon))
  (LocalVariables|SetNewSprite (.WeaponSprite (Utilities|Struct|BreakWeaponStruct _outrow)))
  ;[1 1 1] Change Weapon
  (Variables|Weapon|SetCurrentWeapon NewWeapon)
  (Rendering|Components|Sprite|SetSprite (Variables|Weapon|GetCurrentWeaponSprite) (LocalVariables|GetNewSprite))
  (CallFunction|ResetBlockShooting)
  (return false))

(fn AddHP
  (params (HealthToAdd :type Float%20%28single-precision%29))
  ;[1 1 1] Check if we go over maxHP with the addition
  (if (<= (Variables|Health|GetMaxHP) (+ HealthToAdd (Variables|Health|GetCurrentHP)))
    ;[1 1 1] Change current HP
    (Variables|Health|SetCurrentHP (Variables|Health|GetMaxHP))
    (else
      (Variables|Health|SetCurrentHP (+ HealthToAdd (Variables|Health|GetCurrentHP)))))
  (return))

(fn IsMaxHP
  (return (<= (Variables|Health|GetMaxHP) (Variables|Health|GetCurrentHP))))

(fn GetDatafromWeapon
  (params (NewParam :type Weapons%20Enum))
  (bind _returnvalue (Utilities|GetDataTableRow "/Game/Data/WeaponStats/WeaponData.WeaponData" (Utilities|String|StringToName (Utilities|String|EnumtoString NewParam)))
    (:then
      (return _returnvalue))))

(fn TakeDamage
  (params (Damage :type Float%20%28single-precision%29))
  (Variables|Health|SetCurrentHP (- (Variables|Health|GetCurrentHP) Damage)))