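; 2DGameMode is a game mode that triggers a delayed update of the player character.
; On BeginPlay it sets a non-looping timer of GameUpdateTime, then casts player character 0 to ThePlayer and caches it.
; When the timer fires, UpdateGame calls Update on that cached player once.
; Two other casts to ThePlayer, from the controller and pawn, are left unconnected.
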(event Custom|UpdateGame
  ;[1 1 1] Update all objects
  (Default|Update (Variables|Default|GetThePlayer)))

(event EventBeginPlay
  ;[1 1 1] Start game timer
  (Utilities|Time|SetTimerbyEvent (delegate Custom|UpdateGame) (Variables|Default|GetGameUpdateTime))
  (bind _asthe_player (Utilities|Casting|CastToThePlayer (Game|GetPlayerCharacter 0)))
  (Variables|Default|SetThePlayer _asthe_player))

(fn ConstructionScript)