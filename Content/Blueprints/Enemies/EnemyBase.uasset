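; EnemyBase is a base enemy Blueprint, with fields for health, regen, damage, fire speed, movement speed and idle/run flipbooks.
; GetDataFromEnemy looks up the EnemyDataTable row whose name matches the Enemy enum value.
; The construction script holds logic to copy that row into the stats and CharacterMovement, but it is disconnected and never runs.
; All event graph events, including Update, are empty.
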(event Custom|Update)

(event EventBeginPlay)

(event Collision|EventActorBeginOverlap
  (params (OtherActor :type Actor%20Object%20Reference)))

(event EventTick
  (params (DeltaSeconds :type Float%20%28single-precision%29)))

(fn ConstructionScript)

(fn GetDatafromEnemy
  (params (Enemy :type Enemies%20Enum))
  (bind _returnvalue (Utilities|GetDataTableRow "/Game/Data/DataTables/EnemyDataTable.EnemyDataTable" (Utilities|String|StringToName (Utilities|String|EnumtoString Enemy)))
    (:then
      (return _returnvalue))))