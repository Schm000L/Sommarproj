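; BulletBase is a projectile actor for weapon bullets, drawn as a sprite turned to face its velocity each tick.
; On construction it looks up its Weapon enum's name in the weapon data table to set sprite, initial speed and lifespan.
; Hits on anything other than another BulletBase call OnHitObject, which destroys the bullet.
; The overlap event meant for enemy hits is still an empty stub.
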(event EventBeginPlay)

(event Collision|EventActorBeginOverlap
  (params (OtherActor :type Actor%20Object%20Reference))
  ;[1 1 1] Hit enemy (will fix later)
)

(event EventTick
  (params (DeltaSeconds :type Float%20%28single-precision%29))
  (bind _returnvalue (Transformation|GetActorLocation))
  ;[1 1 1] Rotate bullet towards where its moving
  (Transformation|SetWorldRotation (Variables|Default|GetRenderComponent) (Math|Rotator|FindLookatRotation _returnvalue (+ _returnvalue (Transformation|GetComponentVelocity (Variables|/Script/Engine.MovementComponent|GetUpdatedPrimitive (Variables|Default|GetProjectileMovement))))) false false))

(event Collision|EventHit
  (params (MyComp :type Primitive%20Component%20Object%20Reference) (Other :type Actor%20Object%20Reference) (OtherComp :type Primitive%20Component%20Object%20Reference) (bSelfMoved :type Boolean) (HitLocation :type Vector) (HitNormal :type Vector :default "0, 0, 0") (NormalImpulse :type Vector :default "0, 0, 0") (Hit :type Hit%20Result%20Structure%20%28by%20ref%29))
  ;[1 1 1] Hit non-enemy (wall, bullet etc)
  ;[1 1 1] Check if we hit another bullet
  (if (not (Utilities|ClassIsChildOf (Utilities|GetClass Other) "BulletBase_C"))
    (CallFunction|OnHitObject)))

(fn ConstructionScript
  ;[1 1 1] Constructor-like behavior
  (bind _outrow (CallFunction|GetDatafromWeapon (Variables|Default|GetWeapon)))
  (Rendering|Components|Sprite|SetSprite (Variables|Default|GetRenderComponent) (.BulletSprite (Utilities|Struct|BreakWeaponStruct _outrow)))
  (Variables|/Script/Engine.ProjectileMovementComponent|SetInitialSpeed (Variables|Default|GetProjectileMovement) (.ProjectileSpeed (Utilities|Struct|BreakWeaponStruct _outrow)))
  (Actor|SetLifeSpan (.TimeToLive (Utilities|Struct|BreakWeaponStruct _outrow))))

(fn OnHitObject
  (Actor|DestroyActor))

(fn GetDatafromWeapon
  (params (NewParam :type Weapons%20Enum))
  (bind _returnvalue (Utilities|GetDataTableRow "/Game/Data/DataTables/WeaponDataTable.WeaponDataTable" (Utilities|String|StringToName (Utilities|String|EnumtoString NewParam)))
    (:then
      (return _returnvalue))))

(fn SetWeapon
  (params (NewWeapon :type Weapons%20Enum))
  (CallFunction|SetWeapon NewWeapon))