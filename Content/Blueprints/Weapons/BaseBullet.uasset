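; BaseBullet is a base bullet actor that destroys itself on overlap, on hit, or after a five-second lifetime.
; Overlap and hit events both route into OnHitObject, which only destroys the actor and applies no damage.
; GetDataFromWeapon looks up a WeaponData table row by converting an enum to the row name, and SetWeapon takes a new weapon, though neither is called from the event graph.
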(event EventBeginPlay
  (Utilities|FlowControl|Delay 5.0)
  (Actor|DestroyActor))

(event Collision|EventActorBeginOverlap
  (params (OtherActor :type Actor%20Object%20Reference))
  (CallFunction|OnHitObject))

(event Collision|EventHit
  (params (MyComp :type Primitive%20Component%20Object%20Reference) (Other :type Actor%20Object%20Reference) (OtherComp :type Primitive%20Component%20Object%20Reference) (bSelfMoved :type Boolean) (HitLocation :type Vector) (HitNormal :type Vector :default "0, 0, 0") (NormalImpulse :type Vector :default "0, 0, 0") (Hit :type Hit%20Result%20Structure%20%28by%20ref%29))
  (CallFunction|OnHitObject))

(fn ConstructionScript)

(fn OnHitObject
  (Actor|DestroyActor))

(fn GetDatafromWeapon
  (params (NewParam :type Weapons%20Enum))
  (bind _returnvalue (Utilities|GetDataTableRow "/Game/Data/WeaponStats/WeaponData.WeaponData" (Utilities|String|StringToName (Utilities|String|EnumtoString NewParam)))
    (:then
      (return _returnvalue))))

(fn SetWeapon
  (params (NewWeapon :type Weapons%20Enum))
  (CallFunction|SetWeapon NewWeapon))